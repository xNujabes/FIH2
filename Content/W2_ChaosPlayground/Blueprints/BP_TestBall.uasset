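; BP_TestBall is a physics test projectile in the Chaos playground that reports whether it hits something or passes through at a given launch speed.
; On BeginPlay it applies the CCD toggle to its mesh and sets its velocity along the actor's forward vector.
; A component hit flags and prints "HIT" with the speed; with no hit after a short delay, it prints "TRAVERSÉ" (passed through) instead.
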(event `self.ReceiveBeginPlay`
  (bind _staticmesh (`self.StaticMesh`))
  (`PrimitiveComponent.SetUseCCD` _staticmesh (`self.UseCDD`) "None")
  (`PrimitiveComponent.SetPhysicsLinearVelocity` _staticmesh (* (`self.GetActorForwardVector`) (`self.LaunchSpeed`)) false "None")
  (`KismetSystemLibrary.Delay` 2.0)
  (if (not (`self.HasHit`))
    (`KismetSystemLibrary.PrintString` (`KismetTextLibrary.Conv_TextToString` (`|FormatText` "TRAVERSÉ \n : {speed}" (`self.LaunchSpeed`))))))

(event `self.StaticMesh.OnComponentHit`
  (params (HitComponent :type "PrimitiveComponent Object Reference") (OtherActor :type "Actor Object Reference") (OtherComp :type "PrimitiveComponent Object Reference") (NormalImpulse :type "Vector Structure") (Hit :type "HitResult Structure (by ref)"))
  (set `self.HasHit` true)
  (`KismetSystemLibrary.PrintString` (`KismetTextLibrary.Conv_TextToString` (`|FormatText` "HIT \n : {speed}" (`self.LaunchSpeed`)))))

(fn `UserConstructionScript`)