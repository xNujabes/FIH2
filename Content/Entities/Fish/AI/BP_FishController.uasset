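; BP_FishController is a fish AI controller that turns perceived actors into a blackboard food target.
; On perception updates, it writes any BP_Tank or Eatable-interface actor to the TargetFoodKeyName key.
; A tank also gets its perception stimuli source deactivated and the loop continues, while the first non-tank eatable ends the loop.
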(event `self.FishPerceptionComp.OnPerceptionUpdated`
  (params (UpdatedActors :type "Array of Actor Object Reference (by ref)"))
  (for _array_element UpdatedActors
    (bind _astank (cast `/Game/Entities/BP_Tank` _array_element)
      (:`then`
        (`BlackboardComponent.SetValueAsObject` (`AIBlueprintHelperLibrary.GetBlackboard` null) (`self.TargetFoodKeyName`) _astank)
        (`ActorComponent.SetActive` (`/Game/Entities/BP_Tank.AIPerceptionStimuliSource` _astank) false false))
      (:`CastFailed`
        (if (`KismetSystemLibrary.DoesImplementInterface` _array_element "/Script/FIH2.Eatable")
          (`BlackboardComponent.SetValueAsObject` (`AIBlueprintHelperLibrary.GetBlackboard` null) (`self.TargetFoodKeyName`) _array_element)
          (break))))))

(fn `UserConstructionScript`)